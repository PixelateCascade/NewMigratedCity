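; Enemy character that roams the map via random navmesh points and kills the player on catching them.
; Pawn sensing triggers a one-time approach, blending the view to the enemy, then setting the crawler AnimBP's Caught flag, disabling input, shaking the camera and calling player death.
; Tick plays a laugh on cooldown when the player is near.
; When Chase is set, Tick sends it once to Checkpoint 4 to roam a smaller radius.
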(event `self.ReceiveBeginPlay`
  ;[1 1 1] Begin Play
  ;[1 1 1] Set References
  (bind _outactors (`GameplayStatics.GetAllActorsOfClass` "/Game/Main/Blueprints/Ch_Main.Ch_Main_C"))
  (set `self.MainCharRef` (`|GetArrayItem` _outactors))
  (`self.Roam`))

(event `Roam`
  ;[1 1 1] Roam Map
  (if (not (`self.Chase`))
    (bind _outactors (`GameplayStatics.GetAllActorsOfClass` "Ch_BadGuy_C"))
    (for _array_element _outactors
      (if (== _array_element self)
        (break)))
    (`|AIMoveTo` self (`NavigationSystemV1.K2_GetRandomLocationInNavigableRadius` (`self.K2_GetActorLocation`) 10000.0 null null) null :!label _label
      (:`OnSuccess`
        (`KismetSystemLibrary.Delay` 2.0)
        (goto _label)))))

(event `self.PawnSensing.OnSeePawn`
  (params (Pawn :type "Pawn Object Reference"))
  (bind _returnvalue (`GameplayStatics.GetPlayerCharacter` 0))
  ;[1 1 1] On See Pawn
  (if (== Pawn _returnvalue)
    (`/Engine/EditorBlueprintResources/StandardMacros.DoOnce` false
      (:`Completed`
        (`|AIMoveTo` self (0.0 0.0 0.0) _returnvalue 400.0
          (:`then`
            (`PlayerController.SetViewTargetWithBlend` (`GameplayStatics.GetPlayerController` 0) self 0.5 "VTBlend_Linear" 0.0 false))
          (:`OnSuccess`
            (bind _asab_crawler (cast `/Game/Main/Assets/Characters/Crawl/AB_Crawler` (`SkeletalMeshComponent.GetAnimInstance` (`self.Mesh`))))
            (set `/Game/Main/Assets/Characters/Crawl/AB_Crawler.Caught` true _asab_crawler)
            (`self.DisableInput` (`self.MainCharRef`) (`GameplayStatics.GetPlayerController` 0))
            (`KismetSystemLibrary.Delay` 1.8)
            (`PlayerCameraManager.PlayCameraShake` :`self` (`GameplayStatics.GetPlayerCameraManager` 0) :`ShakeClass` "/Game/Main/Blueprints/BP_CameraShakeDeath.BP_CameraShakeDeath_C")
            ;;[1 1 1] Main Character Death
            (`/Game/Main/Blueprints/Ch_Main.DeathCustomEvent` (`self.MainCharRef`))))))))

(event `self.ReceiveTick`
  (params (DeltaSeconds :type "Float (single-precision)"))
  ;[1 1 1] Event Tick
  (`|ExecutionSequence`
    (:`then_0`
      ;[1 1 1] Play Laugh when in range
      (if (<= (`self.GetDistanceTo` (`self.MainCharRef`)) 2000.0)
        (`/Engine/EditorBlueprintResources/StandardMacros.DoOnce` false :!label _label_2
          (:`Completed`
            (`AudioComponent.Play` (`self.damo_crazy_laugh_Cue`) 0.0)
            (`KismetSystemLibrary.Delay` 19.950001)
            (goto _label_2 :!via `Reset`)))))
    (:`then_1`
      ;[1 1 1] Move to Checkpoint 4
      (if (`self.Chase`)
        (`/Engine/EditorBlueprintResources/StandardMacros.DoOnce` false
          (:`Completed`
            (`KismetSystemLibrary.PrintString` "Chase")
            (bind _outactors (`GameplayStatics.GetAllActorsOfClass` "/Game/Main/Blueprints/BP_Checkpoint4.BP_Checkpoint4_C"))
            (`|AIMoveTo` self (`self.K2_GetActorLocation` (`|GetArrayItem` _outactors)) null
              (:`OnSuccess`
                (`self.Roam Checkpoint 4`)))))))))

(event `Roam Checkpoint 4`
  (bind _returnvalue (`Controller.K2_GetPawn` (`self.GetController`)))
  ;[1 1 1] Roam Checkpoint 4
  (`|AIMoveTo` _returnvalue (`NavigationSystemV1.K2_GetRandomLocationInNavigableRadius` (`self.K2_GetActorLocation` _returnvalue) 3000.0 null null) null :!label _label_3
    (:`OnSuccess`
      (`KismetSystemLibrary.Delay` 2.0)
      (goto _label_3))))

(fn `UserConstructionScript`)
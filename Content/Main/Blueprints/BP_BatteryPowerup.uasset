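; Battery powerup actor that tells the main character (Ch_Main) when it is within pickup range.
; Box overlap begin sets the character's BatteryInRange flag and stores a reference to this powerup, and overlap end clears both.
; Two DoOnce gates reset each other so enter and exit alternate, with debug prints of the reference on each change.
; The pickup effect itself is not handled here.
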(event `self.Box.OnComponentBeginOverlap`
  (params (OverlappedComponent :type "PrimitiveComponent Object Reference") (OtherActor :type "Actor Object Reference") (OtherComp :type "PrimitiveComponent Object Reference") (OtherBodyIndex :type Integer) (bFromSweep :type Boolean) (SweepResult :type "HitResult Structure (by ref)"))
  (bind _asch_main (cast `/Game/Main/Blueprints/Ch_Main` OtherActor))
  (`/Engine/EditorBlueprintResources/StandardMacros.DoOnce` false :!label _label
    (:`Completed`
      (set `/Game/Main/Blueprints/Ch_Main.BatteryInRange` true _asch_main)
      (bind _output_get (set `/Game/Main/Blueprints/Ch_Main.BatteryPowerupRef` self _asch_main))
      (`KismetSystemLibrary.PrintString` (`KismetSystemLibrary.GetDisplayName` _output_get))
      (goto _label_2 :!via `Reset`))))

(event `self.Box.OnComponentEndOverlap`
  (params (OverlappedComponent :type "PrimitiveComponent Object Reference") (OtherActor :type "Actor Object Reference") (OtherComp :type "PrimitiveComponent Object Reference") (OtherBodyIndex :type Integer))
  (bind _asch_main (cast `/Game/Main/Blueprints/Ch_Main` OtherActor))
  (`/Engine/EditorBlueprintResources/StandardMacros.DoOnce` false :!label _label_2
    (:`Completed`
      (set `/Game/Main/Blueprints/Ch_Main.BatteryInRange` false _asch_main)
      (bind _output_get (set `/Game/Main/Blueprints/Ch_Main.BatteryPowerupRef` null _asch_main))
      (`KismetSystemLibrary.PrintString` (`KismetSystemLibrary.GetDisplayName` _output_get))
      (goto _label :!via `Reset`))))

(fn `UserConstructionScript`)
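; BP_Checkpoint2 is a one-shot checkpoint that recharges the player's Power and awards score, then spawns the next checkpoint.
; When Ch_Main overlaps the Cylinder, it plays a recharge sound and starts the Fuel timeline.
; Each update adds to Power, capped at 0.25 above its starting value and at 1.0 overall.
; When the timeline finishes, it spawns BP_Checkpoint3 at a hardcoded transform, adds score and destroys itself.
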(event `self.Cylinder.OnComponentBeginOverlap`
  (params (OverlappedComponent :type "PrimitiveComponent Object Reference") (OtherActor :type "Actor Object Reference") (OtherComp :type "PrimitiveComponent Object Reference") (OtherBodyIndex :type Integer) (bFromSweep :type Boolean) (SweepResult :type "HitResult Structure (by ref)"))
  (bind _asch_main (cast `/Game/Main/Blueprints/Ch_Main` OtherActor))
  (`/Engine/EditorBlueprintResources/StandardMacros.DoOnce` false
    (:`Completed`
      (bind _power (`/Game/Main/Blueprints/Ch_Main.Power` _asch_main))
      (bind _output_get (set `self.PowerLocalVar` _power))
      (`GameplayStatics.PlaySound2D` "/Game/Main/Audio/CheckpointRecharge.CheckpointRecharge" 1.0 1.0 0.0 null null)
      (bind (_direction _newtrack_0) (`Timeline|Fuel` :!via `PlayFromStart`)
        (:`Update`
          (set `/Game/Main/Blueprints/Ch_Main.Power` (`KismetMathLibrary.FClamp` (`KismetMathLibrary.FClamp` (+ _power _newtrack_0) 0.0 (+ _output_get 0.25))) _asch_main))
        (:`Finished`
          (`|SpawnActorFromClass` "/Game/Main/Blueprints/BP_Checkpoint3.BP_Checkpoint3_C" (`KismetMathLibrary.MakeTransform` (-3920.0 -3380.0 1090.0) (struct) (20.0 20.0 50.0)) "Undefined" "OverrideRootScale" null null)
          (set `/Game/Main/Blueprints/Ch_Main.Score` (+ (`/Game/Main/Blueprints/Ch_Main.Score` _asch_main) 250) _asch_main)
          (`self.K2_DestroyActor`))))))

(fn `UserConstructionScript`)
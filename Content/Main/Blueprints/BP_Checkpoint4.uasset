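; Checkpoint actor that recharges the player's Power, awards score and triggers a chase by the Crawler enemy.
; Cylinder overlap by Ch_Main plays a sound and runs a timeline that raises Power, capped at a quarter above its starting value and at full, then adds score and destroys the checkpoint.
; A separate Box overlap, also one-shot, sets Chase on the first Ch_BadGuy found at BeginPlay.
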(event `self.ReceiveBeginPlay`
  (bind _outactors (`GameplayStatics.GetAllActorsOfClass` "/Game/Main/Blueprints/Ch_BadGuy.Ch_BadGuy_C"))
  (set `self.BadGuyRef` (`|GetArrayItem` _outactors)))

(event `self.Cylinder.OnComponentBeginOverlap`
  (params (OverlappedComponent :type "PrimitiveComponent Object Reference") (OtherActor :type "Actor Object Reference") (OtherComp :type "PrimitiveComponent Object Reference") (OtherBodyIndex :type Integer) (bFromSweep :type Boolean) (SweepResult :type "HitResult Structure (by ref)"))
  (bind _asch_main (cast `/Game/Main/Blueprints/Ch_Main` OtherActor))
  (`/Engine/EditorBlueprintResources/StandardMacros.DoOnce` false
    (:`Completed`
      (bind _power (`/Game/Main/Blueprints/Ch_Main.Power` _asch_main))
      (bind _output_get (set `self.PowerLocalVar` _power))
      (`GameplayStatics.PlaySound2D` "/Game/Main/Audio/CheckpointRecharge.CheckpointRecharge" 1.0 1.0 0.0 null null)
      (bind (_direction _float_track) (`Timeline|Timeline_0` :!via `PlayFromStart`)
        (:`Update`
          (set `/Game/Main/Blueprints/Ch_Main.Power` (`KismetMathLibrary.FClamp` (`KismetMathLibrary.FClamp` (+ _power _float_track) 0.0 (+ _output_get 0.25))) _asch_main))
        (:`Finished`
          (set `/Game/Main/Blueprints/Ch_Main.Score` (+ (`/Game/Main/Blueprints/Ch_Main.Score` _asch_main) 250) _asch_main)
          (`self.K2_DestroyActor`))))))

(event `self.Box.OnComponentBeginOverlap`
  (params (OverlappedComponent :type "PrimitiveComponent Object Reference") (OtherActor :type "Actor Object Reference") (OtherComp :type "PrimitiveComponent Object Reference") (OtherBodyIndex :type Integer) (bFromSweep :type Boolean) (SweepResult :type "HitResult Structure (by ref)"))
  ;[1 1 1] Crawler chase within range
  (cast `/Game/Main/Blueprints/Ch_Main` OtherActor)
  (`/Engine/EditorBlueprintResources/StandardMacros.DoOnce` false
    (:`Completed`
      (set `/Game/Main/Blueprints/Ch_BadGuy.Chase` true (`self.BadGuyRef`))
      (`KismetSystemLibrary.PrintString` "Chase True"))))

(fn `UserConstructionScript`)